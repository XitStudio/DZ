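; BP_Balls is an actor that drops a batch of BP_OneBall actors when its Box component is overlapped.
; On overlap it takes the first BP_Area in the level and uses that actor's Count as the number of balls.
; Each ball spawns at a fixed height, at X/Y values read from DT_Location with random jitter, then a debug end message prints.
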(event OnComponentBeginOverlap(Box)
  (params (OverlappedComponent :type Primitive%20Component%20Object%20Reference) (OtherActor :type Actor%20Object%20Reference) (OtherComp :type Primitive%20Component%20Object%20Reference) (OtherBodyIndex :type Integer) (bFromSweep :type Boolean) (SweepResult :type Hit%20Result%20Structure%20%28by%20ref%29))
  (bind _outactors (Actor|GetAllActorsOfClass "/Game/BP/BP_Area.BP_Area_C"))
  (bind _asbp_area (Utilities|Casting|CastToBP_Area (Utilities|Array|Get(acopy) _outactors)))
  (for _index (range 1 (Variables|/Game/BP/BP_Area.BP_Area_C|GetCount _asbp_area))
    (bind _returnvalue (Utilities|GetDataTableRow "/Game/BP/DT_Location.DT_Location" "LocationX")
      (:then
        (bind _returnvalue_2 (Utilities|GetDataTableRow "/Game/BP/DT_Location.DT_Location" "LocationY")
          (:then
            (Game|SpawnActorfromClass "/Game/BP/BP_OneBall.BP_OneBall_C" (Math|Transform|MakeTransform (Math|Vector|MakeVector (+ (Utilities|Struct|BreakBPS_StrLocation _returnvalue) (Math|Random|RandomFloatinRange -5e+01 5e+01)) (+ (Utilities|Struct|BreakBPS_StrLocation _returnvalue_2) (Math|Random|RandomFloatinRange -5e+01 5e+01)) 4e+03) "0, 0, 0" "1.000000,1.000000,1.000000") "Undefined" "MultiplyWithRoot" 0 0))))))
  (Development|PrintString "END!"))

(event EventBeginPlay)

(event Collision|EventActorBeginOverlap
  (params (OtherActor :type Actor%20Object%20Reference)))

(event EventTick
  (params (DeltaSeconds :type Float%20%28single-precision%29)))

(fn ConstructionScript)